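; Player controller that lets the player cycle control between the BP_SkvtBaseChar characters in the level.
; On BeginPlay it adds the default and pawn-swap Enhanced Input mapping contexts.
; The IA_Swap action gathers every base character and possesses the one FindNextCharacter returns.
; That helper picks the entry after the controlled pawn, wrapping to the first, and returns no character if the pawn is not in the list.
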(event Input|EnhancedActionEvents|EnhancedInputActionIA_Swap
  (params (ActionValue :type Boolean) (ElapsedSeconds :type Float%20%28double-precision%29) (TriggeredSeconds :type Float%20%28double-precision%29) (InputAction :type Input%20Action%20Object%20Reference :default "/Game/Skvt/Characters/Input/Actions/IA_Swap.IA_Swap"))
  (bind _outactors (Actor|GetAllActorsOfClass "/Game/Skvt/Characters/BP_SkvtBaseChar.BP_SkvtBaseChar_C"))
  (Pawn|Possess (CallFunction|FindNextCharacter _outactors)))

(event EventBeginPlay
  (bind _self self)
  (bind _returnvalue (PlayerController|LocalPlayerSubsystems|GetEnhancedInputLocalPlayerSubsystem _self))
  (Utilities|IsValid _returnvalue
    (:Is%20Valid
      (Input|AddMappingContext _returnvalue "/Game/Skvt/Characters/Input/IMC_Default.IMC_Default" 0 "(bIgnoreAllPressedKeysUntilRelease=True,bForceImmediately=False,bNotifyUserSettings=False)")
      (Input|AddMappingContext _returnvalue "/Game/Skvt/Characters/Input/IMC_PawnSwap.IMC_PawnSwap" 0 "(bIgnoreAllPressedKeysUntilRelease=True,bForceImmediately=False,bNotifyUserSettings=False)"))))

(fn ConstructionScript)

(fn FindNextCharacter
  (params (All%20Characters :type Array%20of%20Pawn%20Object%20References))
  (bind _returnvalue (Pawn|GetControlledPawn))
  (bind _returnvalue_2 (Utilities|Array|FindItem All%20Characters _returnvalue))
  (bind _returnvalue_3 (+ _returnvalue_2 1))
  (if (>= _returnvalue_2 0)
    (if (== _returnvalue_3 (Utilities|Array|Length All%20Characters))
      (return (Utilities|Array|Get(acopy) All%20Characters))
      (else
        (return (Utilities|Array|Get(acopy) All%20Characters _returnvalue_3))))))